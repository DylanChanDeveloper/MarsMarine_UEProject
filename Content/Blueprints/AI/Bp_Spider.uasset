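; Spider alien enemy that chases the player, plays an attack montage within range and can be killed.
; A looping AIMoveTo retries after each success or failure, while Tick pauses movement during attacks.
; DamagePlayer applies hit damage but is not called within this Blueprint.
; Health reaching exactly zero disables movement and collision, credits the marine's kill, notifies the GameMode and destroys the actor after a delay.
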(event EventBeginPlay
  ;[1 1 1] Movement to player blueprint, if player is outside navmesh and re-enters this code will allow the alien to still move towards the player instead of stopping. The blueprint will first check if the alien is alive then execute.
  (if (CallFunction|IsAlive) :!label _label
    (AI|AIMoveTo self "0, 0, 0" (Game|GetPlayerCharacter 0) 5.0 false
      (:OnSuccess
        _)
      (:OnFail
        _))
    (Utilities|FlowControl|Delay 0.2)
    (goto _label)))

(event EventTick
  (params (DeltaSeconds :type Float%20%28single-precision%29))
  ;[1 1 1] Checks if alien is within attack range and is attacking, stops the a.i movement when attacking and activates it when its not
  (if (CallFunction|CanAttack)
    (CallFunction|DeactivateAIMovment)
    (Animation|Montage|PlayMontage (Variables|Character|GetMesh) "/Game/Characters/Enemy_Great_Spider/Animations/Spider_attack1.Spider_attack1"
      (:OnCompleted
        (CallFunction|ActivateAIMovement)))))

(event Game|Damage|EventAnyDamage
  (params (Damage :type Float%20%28single-precision%29) (DamageType :type Damage%20Type%20Object%20Reference) (InstigatedBy :type Controller%20Object%20Reference) (DamageCauser :type Actor%20Object%20Reference))
  ;[1 1 1] damage the alien blueprint
  (if (CallFunction|IsAlive)
    (bind _health (CallFunction|DecreaseHealth Damage))
    (if (== _health 0.0)
      (CallFunction|KillAI)
      (Utilities|FlowControl|Delay 3.0)
      (Actor|DestroyActor))))

(fn ConstructionScript)

(fn IsWithinAttackRange
  (return (< (Transformation|GetDistanceTo (Game|GetPlayerCharacter 0)) (Variables|Default|GetAttack%20range))))

(fn IsAttacking
  ;[1 1 1] Function tells us if the alien is attacking or not
  (return (Animation|Montage|MontageIsPlaying (Components|SkeletalMesh|GetAnimInstance (Variables|Character|GetMesh)) "/Game/Characters/Enemy_Great_Spider/Animations/Spider_attack1.Spider_attack1")))

(fn DeactivateAIMovment
  (bind _charactermovement (Variables|Character|GetCharacterMovement))
  ;[1 1 1] Deactivates the movement immediatly to stop the spider from looking at the player when it dies, then deactivates the movement
  (Components|Movement|StopMovementImmediately _charactermovement)
  (Components|Activation|Deactivate _charactermovement))

(fn ActivateAIMovement
  (Components|Activation|Activate (Variables|Character|GetCharacterMovement) false))

(fn DamagePlayer
  (if (CallFunction|IsAlive)
    (Game|Damage|ApplyDamage (Game|GetPlayerCharacter 0) (Variables|Default|GetDamage%20per%20hit) 0 0)))

(fn DecreaseHealth
  (params (Damage%20Amount :type Float%20%28double-precision%29))
  (bind _output_get (Variables|Default|SetHealth (- (Variables|Default|GetHealth) Damage%20Amount)))
  (return _output_get))

(fn KillAI
  (Variables|Default|SetDead true)
  (CallFunction|DeactivateAIMovment)
  (Collision|SetActorEnableCollision false)
  (bind _asbp_marine_character (Utilities|Casting|CastToBP_MarineCharacter (Game|GetPlayerCharacter 0)))
  (Default|IncreaseKills _asbp_marine_character)
  (bind _asbp_game_mode (Utilities|Casting|CastToBP_GameMode (Game|GetGameMode)))
  (Default|RegisterAlienDeath _asbp_game_mode self))

(fn IsAlive
  (return (not (Variables|Default|GetDead))))

(fn CanAttack
  (return (Math|Boolean|ANDBoolean (CallFunction|IsWithinAttackRange) (not (CallFunction|IsAttacking)) (CallFunction|IsAlive))))