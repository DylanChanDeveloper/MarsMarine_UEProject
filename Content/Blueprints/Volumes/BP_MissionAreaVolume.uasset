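; BP_MissionAreaVolume is a volume that marks the mission area and punishes the player for leaving it.
; Overlap events toggle OutsideMissionArea on BP_MarineCharacter and start or clear a function-name timer lasting SecondsBeforePlayerDeath.
; When the timer expires, Kill player applies 100 damage to player character 0, regardless of which marine left the volume.
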(event EventBeginPlay)

(event Collision|EventActorBeginOverlap
  (params (OtherActor :type Actor%20Object%20Reference))
  (bind _asbp_marine_character (Utilities|Casting|CastToBP_MarineCharacter OtherActor))
  (Variables|/Game/Blueprints/Pawns/BP_MarineCharacter.BP_MarineCharacter_C|SetOutside%20Mission%20Area _asbp_marine_character false)
  (Utilities|Time|ClearTimerbyFunctionName 0 "Kill player"))

(event EventTick
  (params (DeltaSeconds :type Float%20%28single-precision%29)))

(event Collision|EventActorEndOverlap
  (params (OtherActor :type Actor%20Object%20Reference))
  (bind _asbp_marine_character (Utilities|Casting|CastToBP_MarineCharacter OtherActor))
  (Variables|/Game/Blueprints/Pawns/BP_MarineCharacter.BP_MarineCharacter_C|SetOutside%20Mission%20Area _asbp_marine_character true)
  (Utilities|Time|SetTimerbyFunctionName 0 "Kill player" (Variables|Default|GetSeconds%20before%20player%20death)))

(fn ConstructionScript)

(fn KillPlayer
  (Game|Damage|ApplyDamage (Game|GetPlayerCharacter 0) 1e+02 0 0))