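; Game mode that runs escalating waves of spider aliens and opens the main menu upon reaching the winning wave number.
; Each wave multiplies the alien count by a difficulty factor, then a looping timer spawns spiders at random TargetPoints until the quota is spent.
; RegisterAlienDeath removes aliens from the tracked array, starting the next wave after a short delay once none remain alive or pending.
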(event Custom|Spawn%20wave
  (CallFunction|SpawnAlien))

(event Custom|End%20Wave
  (Utilities|FlowControl|Delay 2.0)
  (CallFunction|StartNewWave))

(event EventBeginPlay
  (Utilities|FlowControl|Delay 2.0)
  (CallFunction|StartNewWave))

(event EventTick
  (params (DeltaSeconds :type Float%20%28single-precision%29)))

(fn ConstructionScript)

(fn StartNewWave
  (Math|Integer|IncrementInt (Variables|Default|GetCurrentWave)
    (:%20%20
      (CallFunction|IncreaseWaveDifficulty)
      (Utilities|Time|SetTimerbyFunctionName 0 "Spawn wave" (Variables|Default|GetSpawn%20Frequency) true)
      (CallFunction|WinWaveCondition))))

(fn SpawnAlien
  (bind _spawn_point (CallFunction|GetRandomSpawnPoint))
  (Utilities|IsValid _spawn_point
    (:Is%20Valid
      (bind _returnvalue (Game|SpawnActorfromClass "/Game/Blueprints/AI/Bp_Spider.Bp_Spider_C" (Transformation|GetActorTransform _spawn_point) "Undefined" 0 0))
      (Utilities|IsValid _returnvalue
        (:Is%20Valid
          (Utilities|Array|Add (Variables|Default|GetAliens) _returnvalue)
          (bind _result (Math|Integer|DecrementInt (Variables|Default|GetAlien%20spawns%20remaining))
            (:%20%20
              (if (== _result 0)
                (Utilities|Time|ClearTimerbyFunctionName 0 "Spawn wave")))))))))

(fn GetRandomSpawnPoint
  (bind _outactors (Actor|GetAllActorsOfClass "/Script/Engine.TargetPoint"))
  (return (Utilities|Array|Get(acopy) _outactors (Math|Random|RandomIntegerinRange 0 (Utilities|Array|LastIndex _outactors)))))

(fn RegisterAlienDeath
  (params (Alien :type Bp%20Spider%20Object%20Reference%20%28by%20ref%29))
  (Utilities|Array|RemoveItem (Variables|Default|GetAliens) Alien)
  (if (CallFunction|IsWaveComplete)
    (CallFunction|EndWave)))

(fn IsWaveComplete
  (return (and (== (Utilities|Array|Length (Variables|Default|GetAliens)) 0) (== (Variables|Default|GetAlien%20spawns%20remaining) 0))))

(fn IncreaseWaveDifficulty
  (bind _output_get (Variables|Default|SetWave%20Difficulty (Math|Float|Round (* (Variables|Default|GetWave%20Difficulty) (Variables|Default|GetDifficulty%20multiplier)))))
  (Variables|Default|SetAlien%20spawns%20remaining _output_get))

(fn WaveCheckforWinCondition
  (Game|OpenLevel(byName) "Mars"))

(fn WinWaveCondition
  (if (== (Variables|Default|GetCurrentWave) (Variables|Default|GetWin%20Wave))
    (Game|OpenLevel(byObjectReference) "/Game/Levels/MainMenu.MainMenu")))