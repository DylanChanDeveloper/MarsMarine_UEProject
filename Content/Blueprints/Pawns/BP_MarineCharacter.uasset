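; Player marine character for a top-down-style shooter, with world-axis movement, a HUD, health and a kill count.
; Aim switches between thumbstick direction and smoothed mouse-velocity direction based on the last key pressed, both deadzoned, setting control-rotation yaw.
; Firing loops effects, sound and a timed muzzle line trace that applies damage and impacts.
; Damage lowers health; exactly zero triggers death, blocking input actions and restarting the level after a delay.
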(event EventBeginPlay
  ;[1 1 1] creates and displays our ui widget
  (bind _returnvalue (UserInterface|CreateWidget "/Game/UI/W_PlayerHUD.W_PlayerHUD_C" 0 self))
  (UserInterface|Viewport|AddtoViewport _returnvalue 0))

(event Game|Damage|EventAnyDamage
  (params (Damage :type Float%20%28single-precision%29) (DamageType :type Damage%20Type%20Object%20Reference) (InstigatedBy :type Controller%20Object%20Reference) (DamageCauser :type Actor%20Object%20Reference))
  ;[1 1 1] player damage blueprints/ player death handling
  (if (CallFunction|IsAlive)
    (bind _health (CallFunction|DecreaseHealth Damage))
    (if (== _health 0.0)
      (Variables|PlayerProperties|SetDead true)
      (Weapon|StopFiringWeapon)
      (Utilities|FlowControl|Delay 3.0)
      (CallFunction|RestartLevel))))

(event EventTick
  (params (DeltaSeconds :type Float%20%28single-precision%29))
  ;[1 1 1] Player aiming blueprint
  (CallFunction|UpdatePlayerAim))

(event Input|ActionEvents|InputActionFireWeapon
  (params (Key :type Key%20Structure :default "None"))
  ;[1 1 1] Weapon blueprint
  (:Pressed
    (Weapon|StartFiringWeapon))
  (:Released
    (Weapon|StopFiringWeapon)))

(event Input|AxisEvents|InputAxisForwardsandBackwards
  (params (AxisValue :type Float%20%28single-precision%29))
  ;[0 0.01271 1] Movement blueprint
  (if (CallFunction|IsAlive)
    (Pawn|Input|AddMovementInput "1.000000, 0, 0" AxisValue false)))

(event Input|AxisEvents|InputAxisLeftandright
  (params (AxisValue :type Float%20%28single-precision%29))
  ;[0 0.01271 1] Movement blueprint
  (if (CallFunction|IsAlive)
    (Pawn|Input|AddMovementInput "0.000000,1.000000, 0" AxisValue false)))

(event Input|KeyboardEvents|AnyKey
  (params (Key :type Key%20Structure :default "None"))
  ;[1 1 1] Funcrionality for telling if the input is mouse or thumbstick
  (:Pressed
    (Variables|Default|Set%20Gamepad%20active (Class|KismetInputLibrary|KeyIsGamepadKey Key))))

(fn ConstructionScript)

(fn UpdatePlayerAim
  ;[1 0.7123 0] Determine input and mouse/thumbstick aiming
  (if (CallFunction|IsAlive)
    (if (Variables|Default|Get%20Gamepad%20active)
      ;;[1 0 0.8581] Aiming blueprint for thumbstick and mouse
      (ThumbstickInput|UpdateThumbstickAim)
      (else
        (MouseInput|UpdateMouseAim)))))

(fn IsThumbstickAboveDeadzone
  (return (> (Math|Vector2D|Vector2DLength (Math|Vector2D|MakeVector2D (Input|AxisValues|GetThumbstickAimUp) (Input|AxisValues|GetThumbstickAimRight))) (Variables|ThumbstickInput|GetThumbstickDeadzone))))

(fn GetMouseVelocity
  (bind _returnvalue (Game|GetPlayerController 0))
  (bind (_deltax _deltay) (Class|PlayerController|GetInputMouseDelta _returnvalue))
  (return (/ (Math|Vector2D|MakeVector2D _deltax _deltay) (Utilities|Time|GetWorldDeltaSeconds))))

(fn IsMouseAboveDeadzone
  (return (> (Math|Vector2D|Vector2DLength (MouseInput|GetMouseVelocity)) (Variables|MouseInput|GetMouse%20Deadzone))))

(fn MouseDeadzoneChallenge
  (return (> (Math|Vector2D|Vector2DLength (MouseInput|GetMouseVelocity)) (Variables|MouseInput|GetMouse%20Deadzone))))

(fn UpdateMouseAim
  (if (MouseInput|IsMouseAboveDeadzone)
    (Pawn|SetControlRotation (Game|GetPlayerController 0) (MouseInput|GetMouseAimDirection))))

(fn GetMouseAimDirection
  (bind _returnvalue (MouseInput|GetMouseVelocity))
  (return (Math|Interpolation|RInterpTo (Pawn|GetControlRotation (Game|GetPlayerController 0) :!class /Script/Engine.Controller) (Math|Rotator|MakeRotator 0.0 0.0 (Class|KismetMathLibrary|DegAtan2 (.x _returnvalue) (.y _returnvalue))) (Utilities|Time|GetWorldDeltaSeconds) (Variables|MouseInput|GetMouse%20Smoothing%20Strength))))

(fn UpdateThumbstickAim
  (if (ThumbstickInput|IsThumbstickAboveDeadzone)
    (Pawn|SetControlRotation (Game|GetPlayerController 0) (ThumbstickInput|GetThumbstickAimDirection))))

(fn GetThumbstickAimDirection
  (return (Math|Rotator|MakeRotator 0.0 0.0 (Class|KismetMathLibrary|DegAtan2 (Input|AxisValues|GetThumbstickAimRight) (Input|AxisValues|GetThumbstickAimUp)))))

(fn StartFiringWeapon
  (if (CallFunction|IsAlive)
    (Components|Activation|Activate (Variables|Default|GetP_AssaultRifle_MF) false)
    (bind _returnvalue (Audio|SpawnSound2D "/Game/Sounds/Weapon_AssaultRifle/Stereo/Rifle_fire_loop.Rifle_fire_loop" 1.0 1.0 0.0 0))
    (Variables|Default|SetWeapon%20fire%20sound _returnvalue)
    (Weapon|WeaponTrace)
    (Utilities|Time|SetTimerbyFunctionName 0 "Weapon trace" (Variables|Weapon|GetWeapon%20fire%20rate) true)))

(fn StopFiringWeapon
  (bind _weapon_fire_sound (Variables|Default|GetWeapon%20fire%20sound))
  (Components|Activation|Deactivate (Variables|Default|GetP_AssaultRifle_MF))
  (Utilities|IsValid _weapon_fire_sound
    (:Is%20Valid
      (Audio|Components|Audio|Stop _weapon_fire_sound)
      (Utilities|Time|ClearTimerbyFunctionName 0 "Weapon trace")
      (if (CallFunction|IsAlive)
        (Audio|SpawnSound2D "/Game/Sounds/Weapon_AssaultRifle/Stereo/RifleFireEnd_Cue.RifleFireEnd_Cue" 1.0 1.0 0.0 0)))))

(fn DecreaseHealth
  (params (Damage%20amount :type Float%20%28double-precision%29))
  (bind _output_get (Variables|playerproperties|SetHealth (- (Variables|playerproperties|GetHealth) Damage%20amount)))
  (return _output_get))

(fn IsAlive
  (return (not (Variables|PlayerProperties|GetDead))))

(fn WeaponTrace
  (bind _outhit (Collision|LineTraceByChannel (Weapon|GetWeaponTraceStartLocation) (Weapon|GetWeaponTraceEndLocation) "TraceTypeQuery1" false 0 "None"))
  (if (.bBlockingHit (Collision|BreakHitResult _outhit))
    (Game|Damage|ApplyDamage (.HitActor (Collision|BreakHitResult _outhit)) (Variables|Weapon|GetDamage%20per%20shot) 0 0)
    (CallFunction|SpawnImpactHit (.Location (Collision|BreakHitResult _outhit)))))

(fn GetWeaponTraceStartLocation
  (return (Transformation|GetSocketLocation (Variables|Default|GetRifle) "MuzzleFlash")))

(fn GetWeaponTraceEndLocation
  (return (+ (Weapon|GetWeaponTraceStartLocation) (* (Math|Vector|GetForwardVector (Pawn|GetControlRotation :!class /Script/Engine.Pawn)) (Variables|Weapon|GetWeapon%20range)))))

(fn IncreaseKills
  (Math|Integer|IncrementInt (Variables|PlayerProperties|Getkills)))

(fn SpawnImpactHit
  (params (Spawn%20location :type Vector))
  (Effects|SpawnEmitteratLocation "/Game/Effects/Weapons/Impacts/P_AssaultRifle_IH.P_AssaultRifle_IH" Spawn%20location))

(fn AddHealth
  (params (health%20to%20add :type Float%20%28double-precision%29))
  (Variables|playerproperties|SetHealth (Math|Float|Clamp(Float) (+ (Variables|playerproperties|GetHealth) health%20to%20add) 0.0 1e+02)))

(fn IsHealthFull
  (return (== (Variables|playerproperties|GetHealth) 1e+02)))

(fn RestartLevel
  (bind _returnvalue (Game|GetCurrentLevelName true))
  (Game|OpenLevel(byName) (Utilities|String|StringToName _returnvalue)))